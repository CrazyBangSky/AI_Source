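; Actor component that steers its owning pawn toward a goal using a direction map from BP_FlowField.
; BeginMovement stores the map and goal, then enables movement.
; Each tick adds constant downward velocity, looks up the pawn's cell direction via FindCurrentCell, and falls back to heading straight at the goal.
; While moving, it smoothly interpolates yaw and adds movement input, stopping within the acceptance distance.
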(event Custom|BeginMovement
  (params (DirectionMap :type Map%20of%20Vector%202D%20Structures%20to%20Structs) (GoalWorldPosition :type Vector))
  ;[1 1 1] Get a direction map and enable movement
  (Variables|Default|SetDirection%20Map DirectionMap)
  (Variables|Default|SetgoalPos GoalWorldPosition)
  (Variables|Default|Setmove? true))

(event EventBeginPlay
  ;[1 1 1] Find the flow field actor
  (bind _returnvalue (Actor|GetActorOfClass "/FlowFieldPathfinding/Blueprints/BP_FlowField.BP_FlowField_C"))
  (Variables|Default|SetFlow%20Field _returnvalue)
  ;[1 1 1] If owner actor is a pawn save it as a variable and find its FloatingPawnMovement component
  (bind _aspawn (Utilities|Casting|CastToPawn (Components|GetOwner)))
  (Variables|Default|SetOwnerPawn _aspawn)
  (Variables|Default|SetFloatingPawnMovement (Actor|GetComponentbyClass _aspawn "/Script/Engine.FloatingPawnMovement")))

(event EventTick
  (params (DeltaSeconds :type Float%20%28single-precision%29))
  (bind _ownerpawn (Variables|Default|GetOwnerPawn))
  (bind _floatingpawnmovement (Variables|Default|GetFloatingPawnMovement))
  (bind _direction_map (Variables|Default|GetDirection%20Map))
  (bind _ownerpawn_2 (Variables|Default|GetOwnerPawn))
  (bind _flow_field (Variables|Default|GetFlow%20Field))
  (bind _ownerpawn_3 (Variables|Default|GetOwnerPawn))
  (bind _returnvalue (Transformation|GetActorLocation _ownerpawn))
  (bind _returnvalue_2 (Transformation|GetActorRotation _ownerpawn_3))
  (bind _celpos (Utilities|FindCurrentCell _returnvalue _flow_field))
  (bind (_value _returnvalue_3) (Utilities|Map|Find _direction_map _celpos))
  ;[1 1 1] Add gravity
  (Variables|/Script/Engine.MovementComponent|SetVelocity _floatingpawnmovement (+ (Variables|/Script/Engine.MovementComponent|GetVelocity _floatingpawnmovement) (* "0,0,-1.000000" 8e+01)))
  ;[1 1 1] Find the direction based on a world position
  (if _returnvalue_3
    (Variables|Default|SetmoveDirection _value)
    (else
      ;[1 1 1] If no direction was found, set the move direction towards the goal world position
      (Variables|Default|SetmoveDirection (Math|Vector|GetUnitDirection(Vector) (Transformation|GetActorLocation (Variables|Default|GetOwnerPawn)) (Variables|Default|GetgoalPos)))))
  ;[1 1 1] Check if the pawn is cloes enough to the goal position
  (if (and (not (<= (Math|Vector|Distance(Vector) (Transformation|GetActorLocation (Variables|Default|GetOwnerPawn)) (Variables|Default|GetgoalPos)) (Variables|Default|GetgoalAcceptenceDist))) (Variables|Default|Getmove?))
    ;[1 1 1] Sets the pawn rotation based on the move direction
    (Transformation|SetActorRotation _ownerpawn_2 (Math|Rotator|MakeRotator (.roll _returnvalue_2) (.pitch _returnvalue_2) (Math|Interpolation|FInterpTo (.yaw _returnvalue_2) (.yaw (Math|Rotator|MakeRotfromX (Variables|Default|GetmoveDirection))) (Utilities|Time|GetWorldDeltaSeconds) 5.0)))
    ;[1 1 1] Add movement towards the Move Direction
    (Pawn|Input|AddMovementInput _ownerpawn_2 (Variables|Default|GetmoveDirection) 1.0 false)
    (else
      ;[1 1 1] Set move = false if pawn is close to goal position
      (Variables|Default|Setmove? false))))