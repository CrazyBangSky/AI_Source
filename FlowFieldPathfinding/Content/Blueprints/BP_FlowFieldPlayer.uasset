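; RTS-style camera player that box-selects pawns and sends them to a clicked goal through BP_FlowField.
; Right-mouse drag pans at a speed scaled to spring arm length, which the mouse wheel zooms.
; Left-mouse drag sizes a box from cursor traces and, on release, gathers overlapped pawns' AC_FlowFieldAIMovement components.
; With a selection active, clicking generates one flow field, passes its direction map to every component, then clears the selection.
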(event EventBeginPlay
  (bind _returnvalue (Game|GetPlayerController 0))
  ;[1 1 1] Event Begin Play: Set input mode game and UI
  (Input|SetInputModeGameandUI _returnvalue 0 "DoNotLock" false)
  (Variables|/Script/Engine.PlayerController|SetbShowMouseCursor _returnvalue true)
  ;;[1 1 1] Find the flow field and save it in a variable
  (bind _returnvalue_2 (Actor|GetActorOfClass "/FlowFieldPathfinding/Blueprints/BP_FlowField.BP_FlowField_C"))
  (Variables|Default|SetFlowFieldActor _returnvalue_2)
  (Variables|Default|SetpanSpeed (/ (Variables|/Script/Engine.SpringArmComponent|GetTargetArmLength (Variables|Default|GetSpringArm)) 5e+02)))

(event EventTick
  (params (DeltaSeconds :type Float%20%28single-precision%29))
  ;[1 1 1] Event Tick
  (Utilities|FlowControl|Sequence
    (:then_0
      (if (Variables|Default|GetrightMouseButtonDown?)
        (Utilities|FlowControl|Sequence
          (:then_0
            ;;[1 1 1] Player Pan Movement
            (Transformation|SetActorLocation (+ (Transformation|GetActorLocation) (* (Transformation|GetActorRightVector) (* (* (Class|Actor|GetInputAxisKeyValue) (Variables|Default|GetpanSpeed)) -2.0))) false false))
          (:then_1
            (Transformation|SetActorLocation (+ (Transformation|GetActorLocation) (* (Transformation|GetActorForwardVector) (* (* (Class|Actor|GetInputAxisKeyValue) (Variables|Default|GetpanSpeed)) -2.0))) false false)))))
    (:then_2
      ;;[1 1 1] Create a selection box
      (if (Variables|Default|GetfoundStartPos?)
        (bind _hitresult (CallFunction|LinetracefromCamera 4e+04 "None"))
        (if (.bBlockingHit (Collision|BreakHitResult _hitresult))
          (Variables|Default|SetendPos (.ImpactPoint (Collision|BreakHitResult _hitresult)))
          (CallFunction|CreateSelectionBox (Variables|Default|GetstartPos) (Variables|Default|GetendPos) 6e+02))))))

(event Input|MouseEvents|RightMouseButton
  (params (Key :type Key%20Structure :default "None"))
  ;[1 1 1] Set player inputs
  (:Pressed
    (Variables|Default|SetrightMouseButtonDown? true)
    (Input|SetInputModeGameOnly (Game|GetPlayerController 0)))
  (:Released
    (Variables|Default|SetrightMouseButtonDown? false)
    (Input|SetInputModeGameandUI (Game|GetPlayerController 0) 0 "DoNotLock" false)))

(event Input|MouseEvents|LeftMouseButton
  (params (Key :type Key%20Structure :default "None"))
  (bind _flowfieldactor (Variables|Default|GetFlowFieldActor))
  (bind _box_visual_ (Variables|Default|GetBox%28Visual%29))
  (bind _box_visual__2 (Variables|Default|GetBox%28Visual%29))
  (bind _returnvalue (Transformation|GetWorldLocation _box_visual_))
  ;[1 1 1] Left mouse button Event
  (:Pressed
    ;;[1 1 1] Start selecting:
    (bind _hitresult (CallFunction|LinetracefromCamera 4e+04 "None"))
    (if (.bBlockingHit (Collision|BreakHitResult _hitresult))
      (if (Utilities|Array|IsNotEmpty (Variables|Default|GetAllFlowFieldComponents))
        ;;[1 1 1] If Player had pawns selected, generate a Flow Field based on a goal and output a direction map to the selected pawns
        (bind (_directionmap _goalworldpos) (Class|FlowFieldCPP|GenerateFlowField _flowfieldactor (Variables|/FlowFieldPathfinding/Blueprints/BP_FlowField.BP_FlowField_C|GetGrid%20Cells _flowfieldactor) (.ImpactPoint (Collision|BreakHitResult _hitresult))))
        (Transformation|SetWorldLocation (Variables|Default|GetSM_GoalMesh) _goalworldpos false false)
        (for _array_element (Variables|Default|GetAllFlowFieldComponents)
          (Default|BeginMovement _array_element _directionmap _goalworldpos))
        (CallFunction|ClearSelectedActors)
        (else
          (Variables|Default|SetfoundStartPos? true)
          (Variables|Default|SetstartPos (.ImpactPoint (Collision|BreakHitResult _hitresult)))))
      (else
        (Variables|Default|SetfoundStartPos? false)
        (CallFunction|ClearSelectedActors))))
  (:Released
    (Utilities|FlowControl|Sequence
      (:then_0
        ;;[1 1 1] Stop Selecting: box trace all pawns in the selected area
        (if (Variables|Default|GetfoundStartPos?)
          (bind _outhits (Class|KismetSystemLibrary|BoxTraceMultiforObjects _returnvalue _returnvalue (Math|Vector|VectorGetAbs (Variables|/Script/Engine.BoxComponent|GetBoxExtent _box_visual_)) "0, 0, 0" (Utilities|Array|MakeArray "ObjectTypeQuery3") false 0 "None" true))
          ;;[1 1 1] Add all selected pawns in an array
          (for _array_element_2 _outhits
            (Utilities|IsValid (Actor|GetComponentbyClass (.HitActor (Collision|BreakHitResult _array_element_2)) "/FlowFieldPathfinding/Blueprints/AC_FlowFieldAIMovement.AC_FlowFieldAIMovement_C")
              (:Is%20Valid
                (Utilities|Array|Add (Variables|Default|GetAllFlowFieldComponents) (Actor|GetComponentbyClass (.HitActor (Collision|BreakHitResult _array_element_2)) "/FlowFieldPathfinding/Blueprints/AC_FlowFieldAIMovement.AC_FlowFieldAIMovement_C")))))))
      (:then_1
        ;;[1 1 1] Reset the selection box
        (Variables|Default|SetfoundStartPos? false)
        (Transformation|SetWorldLocation _box_visual__2 "0, 0,100000.000000" false false)
        (Components|Box|SetBoxExtent _box_visual__2 "0, 0, 0" false)))))

(event Input|MouseEvents|MouseWheelDown
  (params (Key :type Key%20Structure :default "None"))
  (bind _springarm (Variables|Default|GetSpringArm))
  ;[1 1 1] Zoom in and out
  (:Pressed
    (Variables|/Script/Engine.SpringArmComponent|SetTargetArmLength _springarm (Math|Float|Clamp(Float) (+ (Variables|/Script/Engine.SpringArmComponent|GetTargetArmLength _springarm) 2e+02) 2e+02 2e+04))
    (Variables|Default|SetpanSpeed (/ (Variables|/Script/Engine.SpringArmComponent|GetTargetArmLength (Variables|Default|GetSpringArm)) 5e+02))))

(event Input|MouseEvents|MouseWheelUp
  (params (Key :type Key%20Structure :default "None"))
  (bind _springarm (Variables|Default|GetSpringArm))
  ;[1 1 1] Zoom in and out
  (:Pressed
    (Variables|/Script/Engine.SpringArmComponent|SetTargetArmLength _springarm (Math|Float|Clamp(Float) (- (Variables|/Script/Engine.SpringArmComponent|GetTargetArmLength _springarm) 2e+02) 2e+02 2e+04))
    (Variables|Default|SetpanSpeed (/ (Variables|/Script/Engine.SpringArmComponent|GetTargetArmLength (Variables|Default|GetSpringArm)) 5e+02))))

(fn ConstructionScript)

(fn LinetracefromCamera
  (params (Distance :type Float%20%28single-precision%29) (DrawDebugType :type EDrawDebugTrace%20Enum :default "None"))
  (bind _camera (Variables|Default|GetCamera))
  (bind _returnvalue (Transformation|GetWorldLocation _camera))
  (bind _outhit (Collision|LineTraceByChannel _returnvalue (+ _returnvalue (* (.WorldDirection (Game|Player|ConvertMouseLocationToWorldSpace (Game|GetPlayerController 0))) Distance)) "TraceTypeQuery1" false 0 DrawDebugType))
  (return _outhit))

(fn ClearSelectedActors
  (Utilities|Array|Clear (Variables|Default|GetAllFlowFieldComponents)))

(fn CreateSelectionBox
  (params (startPos :type Vector) (endPos :type Vector) (BoxHeight :type Float%20%28double-precision%29))
  (bind _returnvalue (/ BoxHeight 2.0))
  (bind _returnvalue_2 (- endPos startPos))
  (bind _box_visual_ (Variables|Default|GetBox%28Visual%29))
  (bind _returnvalue_3 (/ _returnvalue_2 2.0))
  (bind _returnvalue_4 (+ startPos _returnvalue_3 (Math|Vector|MakeVector 0.0 0.0 _returnvalue)))
  (bind (_x _y) (Math|Vector|BreakVector _returnvalue_4))
  (bind _returnvalue_5 (- _returnvalue_4 startPos))
  (bind (_x_2 _y_2) (Math|Vector|BreakVector _returnvalue_5))
  (Transformation|SetWorldLocation _box_visual_ (Math|Vector|MakeVector _x _y (.Z (Math|Vector|BreakVector startPos))) false false)
  (Components|Box|SetBoxExtent _box_visual_ (Math|Vector|MakeVector _x_2 _y_2 BoxHeight) false))